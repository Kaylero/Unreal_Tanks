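; Player-controllable tank pawn that wires up aiming, track-driven movement and a health bar widget.
; On BeginPlay it sets the projectile class, hands barrel and turret to the aiming component and both tracks to the movement component.
; Axis inputs rotate the azimuth gimbal and spring arm for camera aim and pass move and turn intent to movement; left mouse fires through aiming.
; The health bar widget receives a reference to this tank.
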(event `self.ReceiveBeginPlay`
  (set `TankAimingComponet.ProjectileBlueprint` "/Game/Projectile/Projectile_BP.Projectile_BP_C" (`self.TankAimingComponet`))
  (`TankAimingComponet.Initialise` (`self.TankAimingComponet`) (`self.Barrel`) (`self.Turret`))
  (`TankMovementComponent.Initialise` (`self.TankMovement`) (`self.LeftTrack`) (`self.RightTrack`))
  (`self.InitialiseHealthbarWidget`))

(event `InputAxis|AimAzimuth`
  (params (AxisValue :type "Float (single-precision)"))
  ;[1 1 1] Aiming Input Binding
  (`SceneComponent.K2_AddLocalRotation` (`self.Azimuth Gimbal`) (`KismetMathLibrary.MakeRotator` 0.0 0.0 AxisValue) false false))

(event `InputAxis|MoveForward`
  (params (AxisValue :type "Float (single-precision)"))
  ;[1 1 1] Movement Input Binding
  (`TankMovementComponent.IntendMoveForward` (`self.TankMovement`) AxisValue))

(event `InputAxis|AimElevation`
  (params (AxisValue :type "Float (single-precision)"))
  ;[1 1 1] Aiming Input Binding
  (`SceneComponent.K2_AddLocalRotation` (`self.SpringArm`) (`KismetMathLibrary.MakeRotator` 0.0 AxisValue) false false))

(event `InputAxis|Turn Right`
  (params (AxisValue :type "Float (single-precision)"))
  ;[1 1 1] Movement Input Binding
  (`TankMovementComponent.IntendTurnRight` (`self.TankMovement`) AxisValue))

(event `Key|LeftMouseButton`
  (params (Key :type "Key Structure"))
  ;[1 1 1] Aiming Input Binding
  (:`Pressed`
    (`TankAimingComponet.Fire` (`self.TankAimingComponet`))))

(fn `InitialiseHealthbarWidget`
  (bind _ashealth_bar (cast `/Game/Blueprints/UI/HealthBar` (`WidgetComponent.GetUserWidgetObject` (`self.HealthBar`))))
  (set `/Game/Blueprints/UI/HealthBar.Tank` self _ashealth_bar))

(fn `UserConstructionScript`)